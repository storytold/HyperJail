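; Star dome actor that renders a configurable nebula and starfield sky on its Dome mesh.
; The construction script creates a dynamic instance of M_Star_Nebula and feeds it flow map, main and extra cubemap, and near and far star textures.
; Exposed variables then drive star intensity and desaturation, per-cubemap tint, brightness and saturation, flow direction, cubemap rotation and sun masking.
; It has no runtime logic.
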(fn `UserConstructionScript`
  (bind _returnvalue (`PrimitiveComponent.CreateDynamicMaterialInstance` (`self.Dome`) 0 "/Game/Space_Construction/Planet_System/Materials/Star_Dome/M_Star_Nebula.M_Star_Nebula" "None"))
  ;[1 1 1] Set_Textures
  (`MaterialInstanceDynamic.SetTextureParameterValue` _returnvalue "Flow_map" (`self.T_Flow_Map`))
  (`MaterialInstanceDynamic.SetTextureParameterValue` _returnvalue "T_Color" (`self.T_Cubemap_Color`))
  (`MaterialInstanceDynamic.SetTextureParameterValue` _returnvalue "T_Alpha" (`self.T_Cubemap_Alpha`))
  (`MaterialInstanceDynamic.SetTextureParameterValue` _returnvalue "T_Color_Extra_Cubemap" (`self.T_ExtraCubemap_Color`))
  (`MaterialInstanceDynamic.SetTextureParameterValue` _returnvalue "T_Alpha_Extra_Cubemap" (`self.T_ExtraCubemap_Alpha`))
  (`MaterialInstanceDynamic.SetTextureParameterValue` _returnvalue "T_Stars_Near" (`self.T_Near_Stars`))
  (`MaterialInstanceDynamic.SetTextureParameterValue` _returnvalue "T_Stars_Far" (`self.T_Far_Stars`))
  ;[1 1 1] Star_Control
  (`MeshComponent.SetScalarParameterValueOnMaterials` (`self.Dome`) "Near_Stars_Desaturation" (`self.Near Star Desaturation`))
  (`MeshComponent.SetScalarParameterValueOnMaterials` (`self.Dome`) "Far_Stars_Desaturation" (`self.Far Star Desaturation`))
  (`MeshComponent.SetScalarParameterValueOnMaterials` (`self.Dome`) "Near_Stars_intensity" (`self.Near_Stars_intensity`))
  (`MeshComponent.SetScalarParameterValueOnMaterials` (`self.Dome`) "Far_Stars_intensity" (`self.Far_Stars_intensity`))
  ;[1 1 1] Color_Control
  (`MeshComponent.SetScalarParameterValueOnMaterials` (`self.Dome`) "Red_Level" (`self.Red Tint`))
  (`MeshComponent.SetScalarParameterValueOnMaterials` (`self.Dome`) "Green_Level" (`self.Green Tint`))
  (`MeshComponent.SetScalarParameterValueOnMaterials` (`self.Dome`) "Blue_Level" (`self.Blue Tint`))
  ;[1 1 1] Color_Control_Extra_Cubemap
  (`MeshComponent.SetScalarParameterValueOnMaterials` (`self.Dome`) "Red_Level_Extra_Cubemap" (`self.Red_Level_Extra_Cubemap`))
  (`MeshComponent.SetScalarParameterValueOnMaterials` (`self.Dome`) "Green_Level_Extra_Cubemap" (`self.Green_Level_Extra_Cubemap`))
  (`MeshComponent.SetScalarParameterValueOnMaterials` (`self.Dome`) "Blue_Level_Extra_Cubemap" (`self.Blue_Level_Extra_Cubemap`))
  ;[1 1 1] Visibility_Control
  (`MeshComponent.SetScalarParameterValueOnMaterials` (`self.Dome`) "Power" (`self.Brightness`))
  (`MeshComponent.SetScalarParameterValueOnMaterials` (`self.Dome`) "Saturation" (`self.Saturation`))
  (`MeshComponent.SetVectorParameterValueOnMaterials` (`self.Dome`) "Flow_Direction" (`self.Flow_Direction`))
  (`MeshComponent.SetScalarParameterValueOnMaterials` (`self.Dome`) "Sun_Mask_Intensity" (`self.Sun_Mask_Threshold`))
  ;[1 1 1] Visibility_Extra_Cubemap
  (`MeshComponent.SetScalarParameterValueOnMaterials` (`self.Dome`) "Saturation_Extra_Cubemap" (`self.Saturation_Extra_Cubemap`))
  (`MeshComponent.SetScalarParameterValueOnMaterials` (`self.Dome`) "Power_Extra_Cubemap" (`self.Brightness_Extra_Cubemap`))
  (`MeshComponent.SetScalarParameterValueOnMaterials` (`self.Dome`) "Cubemap_Rotation" (`self.Cubemap_Rotation`)))